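; NPC population manager that shows each NPC's mood and health visually through material swaps.
; A mood change handler sets the first material slot of the NPC's mesh to a material matching that mood.
; A health change handler casts to BP_NPCCharacter and sets the Face component's material for the new state, using a dead material for Critical.
; Both react only to the change events, with no Tick logic.
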(event EventBeginPlay)

(event Collision|EventActorBeginOverlap
  (params (OtherActor :type Actor%20Object%20Reference)))

(event EventTick
  (params (DeltaSeconds :type Float%20%28single-precision%29)))

(event EventHandleMoodChanged
  (params (NPC :type NPC%20Character%20Object%20Reference) (Mood :type EMoodState%20Enum :default "Overjoyed"))
  (Variables|Default|SetMesh (Variables|/Script/Engine.Character|GetMesh NPC))
  (switch Utilities|FlowControl|Switch|SwitchonEMoodState Mood
    (:Overjoyed
      (Rendering|Material|SetMaterial (Variables|Default|GetMesh) 0 "/Game/Artifact/Materials/M_Overjoyed.M_Overjoyed"))
    (:Happy
      (Rendering|Material|SetMaterial (Variables|Default|GetMesh) 0 "/Game/Artifact/Materials/M_Happy.M_Happy"))
    (:Fine
      (Rendering|Material|SetMaterial (Variables|Default|GetMesh) 0 "/Game/Artifact/Materials/M_Fine.M_Fine"))
    (:Sad
      (Rendering|Material|SetMaterial (Variables|Default|GetMesh) 0 "/Game/Artifact/Materials/M_Sad.M_Sad"))
    (:Depressed
      (Rendering|Material|SetMaterial (Variables|Default|GetMesh) 0 "/Game/Artifact/Materials/M_Depressed.M_Depressed"))))

(event EventHandleHealthChanged
  (params (NPC :type NPC%20Character%20Object%20Reference) (Health :type EHealthState%20Enum :default "Healthy"))
  (bind _asbp_npccharacter (Utilities|Casting|CastToBP_NPCCharacter NPC))
  (Variables|Default|SetFace (Variables|/Game/Artifact/Blueprints/BP_NPCCharacter.BP_NPCCharacter_C|GetFace _asbp_npccharacter))
  (switch Utilities|FlowControl|Switch|SwitchonEHealthState Health
    (:Healthy
      (Rendering|Material|SetMaterial (Variables|Default|GetFace) 0 "/Game/Artifact/Images/Healthy_Mat.Healthy_Mat"))
    (:Injured
      (Rendering|Material|SetMaterial (Variables|Default|GetFace) 0 "/Game/Artifact/Images/Injured_Mat.Injured_Mat"))
    (:Sick
      (Rendering|Material|SetMaterial (Variables|Default|GetFace) 0 "/Game/Artifact/Images/Sick_Mat.Sick_Mat"))
    (:Critical
      (Rendering|Material|SetMaterial (Variables|Default|GetFace) 0 "/Game/Artifact/Images/Dead_Mat.Dead_Mat"))))

(fn ConstructionScript)